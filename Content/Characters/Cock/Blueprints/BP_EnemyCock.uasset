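; BP_EnemyCock is the enemy rooster whose death wins the game.
; BeginPlay caches the BP_PlayerCock reference, looping back immediately until it is valid.
; HitReact, gated by IsGettingHit, plays a hit montage and subtracts the player's AttackStat from Health, rechecking Health when the montage completes or is interrupted.
; At zero Health it ragdolls, drops capsule collision, then after a delay shows W_WinScreen and freezes time via global time dilation.
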(event `self.ReceiveBeginPlay`
  (bind _returnvalue (`GameplayStatics.GetActorOfClass` "/Game/Characters/Cock/Blueprints/BP_PlayerCock.BP_PlayerCock_C" :!label _label))
  (bind _output_get (set `self.Player` _returnvalue))
  (`/Engine/EditorBlueprintResources/StandardMacros.IsValid` _output_get
    (:`Is Not Valid`
      (goto _label))))

(event `self.HitReact`
  (if (not (`self.isGettingHit`))
    (set `self.isGettingHit` true)
    (`|PlayMontage` (`self.Mesh`) "/Game/Characters/Cock/Animations/Chicken_GetHit_Anim_Montage.Chicken_GetHit_Anim_Montage" 1.5
      (:`then`
        (bind _output_get (set `self.Health` (- (`self.Health`) (`/Game/Characters/Cock/Blueprints/BP_PlayerCock.AttackStat` (`self.Player`))))))
      (:`OnCompleted`
        _)
      (:`OnInterrupted`
        _))
    (if (<= (`self.Health`) 0)
      (`PrimitiveComponent.SetSimulatePhysics` (`self.Mesh`) true)
      (`PrimitiveComponent.SetCollisionEnabled` (`self.CapsuleComponent`) "NoCollision")
      (`self.SetActorTickEnabled` false)
      (`KismetSystemLibrary.Delay` 3.0)
      (bind _returnvalue (`|CreateWidget` "/Game/Widgets/W_WinScreen.W_WinScreen_C"))
      (`UserWidget.AddToViewport` _returnvalue 0)
      (`GameplayStatics.SetGlobalTimeDilation` 0.0)
      (else
        (`KismetSystemLibrary.Delay` 0.7)
        (set `self.isGettingHit` false)))))

(fn `UserConstructionScript`
  (`parent.UserConstructionScript`))