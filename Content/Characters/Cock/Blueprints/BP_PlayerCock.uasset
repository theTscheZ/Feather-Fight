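; Player rooster character for a melee fighting game, with Enhanced Input, health and attack stats, and buff and reset functions.
; Light attack plays a pick, wing-slap or kick montage by combo count.
; HitDetect sphere-traces at that attack's bone socket and triggers HitReact on another BP_PlayerCock.
; HitReact deals fixed damage, ignoring AttackStat; at zero health it ragdolls, shows the lose screen and freezes time.
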(event `self.ReceiveBeginPlay`
  (`self.SetupInput`))

(event `SetupInput`
  (bind _asplayer_controller (cast `PlayerController` (`self.GetController`)))
  (bind _returnvalue (pcsubsystem `EnhancedInputLocalPlayerSubsystem` _asplayer_controller))
  (`/Engine/EditorBlueprintResources/StandardMacros.IsValid` _returnvalue
    (:`Is Valid`
      (`EnhancedInputSubsystemInterface.AddMappingContext` _returnvalue "/Game/Characters/Cock/Input/IMC_FeatherFight.IMC_FeatherFight" 0 (struct))
      (`EnhancedInputSubsystemInterface.AddMappingContext` _returnvalue "/Game/ThirdPerson/Input/IMC_Default.IMC_Default" 0 (struct)))))

(event `EnhancedInput|/Game/Characters/Cock/Input/IA_LightAtk`
  (params (ActionValue :type Boolean) (ElapsedSeconds :type "Float (double-precision)") (TriggeredSeconds :type "Float (double-precision)") (InputAction :type "InputAction Object Reference" :default "/Game/Characters/Cock/Input/IA_LightAtk.IA_LightAtk"))
  (:`Started`
    (`self.Attack`)))

(event `Attack`
  (if (`self.isGettingHit`)
    _
    (elif (not (`self.isAttacking`))
      (set `self.isAttacking` true)
      (`|PlayMontage` (`self.Mesh`) (select `int` (`self.AtkCount`) :`0` "/Game/Characters/Cock/Animations/Chicken_pick__attack_Anim_root_rootAction_Montage.Chicken_pick__attack_Anim_root_rootAction_Montage" :`1` "/Game/Characters/Cock/Animations/Chicken_fluegelslap_Anim_root_rootAction_Montage.Chicken_fluegelslap_Anim_root_rootAction_Montage" :`2` "/Game/Characters/Cock/Animations/Chicken_kick_Anim_root_rootAction_Montage.Chicken_kick_Anim_root_rootAction_Montage" :!type "AnimMontage Object Reference") 1.5
        (:`then`
          (`/Engine/EditorBlueprintResources/StandardMacros.IncrementInt` (`self.AtkCount`)))
        (:`OnCompleted`
          (set `self.AtkCount` 0 :!label _label))
        (:`OnInterrupted`
          (`KismetSystemLibrary.RetriggerableDelay` 0.77)
          (set `self.isAttacking` false)
          (goto _label))))))

(event `HitReact`
  (if (not (`self.isGettingHit`))
    (set `self.isGettingHit` true)
    (`|PlayMontage` (`self.Mesh`) "/Game/Characters/Cock/Animations/Chicken_GetHit_Anim_Montage.Chicken_GetHit_Anim_Montage" 1.5
      (:`then`
        (set `self.Health` (- (`self.Health`) 5)))
      (:`OnCompleted`
        _)
      (:`OnInterrupted`
        _))
    (if (<= (`self.Health`) 0)
      (`PrimitiveComponent.SetSimulatePhysics` (`self.Mesh`) true)
      (`PrimitiveComponent.SetCollisionEnabled` (`self.CapsuleComponent`) "NoCollision")
      (`self.DisableInput` (`GameplayStatics.GetPlayerController` 0))
      (`KismetSystemLibrary.Delay` 3.0)
      (bind _returnvalue (`|CreateWidget` "/Game/Widgets/W_LoseScreen.W_LoseScreen_C"))
      (`UserWidget.AddToViewport` _returnvalue 0)
      (`GameplayStatics.SetGlobalTimeDilation` 0.0)
      (else
        (`KismetSystemLibrary.Delay` 0.5)
        (set `self.isGettingHit` false)))))

(event `Reset`
  (`self.ResetLevelDispatcher`))

(fn `AttackBuff`
  (params (`Attack Buff` :type Integer))
  (set `self.AttackStat` (+ (`self.AttackStat`) `Attack Buff`)))

(fn `HealthBuff`
  (params (HealthBuff :type Integer))
  (set `self.Health` (+ (`self.Health`) HealthBuff)))

(fn `HitDetect`
  (bind _returnvalue (`SceneComponent.GetSocketLocation` (`self.Mesh`) (select `int` (- (`self.AtkCount`) 1) :`0` "Bone" :`1` "Bone_016_l" :`2` "Bone_008_r" :!type "Name")))
  (if (== (`self.AtkCount`) 3)
    (set `self.Radius` 100.0)
    (else
      (set `self.Radius` 42.0)))
  (bind _outhit (`KismetSystemLibrary.SphereTraceSingleForObjects` _returnvalue _returnvalue (`self.Radius`) (`|MakeArray` "ObjectTypeQuery3" :!type "EObjectTypeQuery Enum")))
  (bind _asbp_player_cock (cast `/Game/Characters/Cock/Blueprints/BP_PlayerCock` (`.HitActor` (`GameplayStatics.BreakHitResult` _outhit))))
  (`self.HitReact` _asbp_player_cock))

(fn `Reset Stats`
  (set `self.AttackStat` 10)
  (set `self.Health` 100))

(fn `UserConstructionScript`)